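; Large hazard barrel that explodes when the first-person character or one of its projectiles overlaps its barrel volume.
; Exploding swaps collision from the barrel to the explosion volume, spawns a particle effect, hides the mesh, and destroys the actor after a timed duration.
; The explosion volume starts the player's large-barrel freeze effect when the character's Sphere enters it.
; End overlap also calls BeginEffect rather than ending the effect.
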(event `DestroyEffect`
  ;[1 1 1] Visual
)

(event `DoParticleEffect`
  ;[1 1 1] Visual
)

(event `BeginExplosion`
  (bind (_returnvalue_x _returnvalue_y _returnvalue_z) (`KismetMathLibrary.BreakVector` (`self.K2_GetActorLocation`)))
  (`PrimitiveComponent.SetCollisionEnabled` (`self.Explosion_Volume`) "QueryAndPhysics")
  (`PrimitiveComponent.SetCollisionEnabled` (`self.Barrel_Volume`) "NoCollision")
  (`PrimitiveComponent.SetCollisionEnabled` (`self.Barrel`) "NoCollision")
  (`GameplayStatics.SpawnEmitterAtLocation` "/Game/StarterContent/Particles/P_Explosion.P_Explosion" (`KismetMathLibrary.MakeVector` _returnvalue_x _returnvalue_y (+ _returnvalue_z 50.0)))
  (`SceneComponent.SetVisibility` (`self.Barrel`) false false)
  (`KismetSystemLibrary.K2_SetTimerDelegate` (delegate `EndExplosion`) (`self.ExplosionDuration`)))

(event `self.Barrel_Volume.OnComponentBeginOverlap`
  (params (OverlappedComponent :type "PrimitiveComponent Object Reference") (OtherActor :type "Actor Object Reference") (OtherComp :type "PrimitiveComponent Object Reference") (OtherBodyIndex :type Integer) (bFromSweep :type Boolean) (SweepResult :type "HitResult Structure (by ref)"))
  ;[1 1 1] When the explosion happens
  (cast `/Game/FirstPersonBP/Blueprints/FirstPersonCharacter` OtherActor
    (:`then`
      _)
    (:`CastFailed`
      (cast `/Game/FirstPersonBP/Blueprints/FirstPersonProjectile` OtherActor)))
  (`self.BeginExplosion`))

(event `DuringExplosion`)

(event `EndExplosion`
  (`self.K2_DestroyActor`))

(event `self.Explosion_Volume.OnComponentBeginOverlap`
  (params (OverlappedComponent :type "PrimitiveComponent Object Reference") (OtherActor :type "Actor Object Reference") (OtherComp :type "PrimitiveComponent Object Reference") (OtherBodyIndex :type Integer) (bFromSweep :type Boolean) (SweepResult :type "HitResult Structure (by ref)"))
  ;[1 1 1] When the player is affected by the explostion
  (bind _asfirst_person_character (cast `/Game/FirstPersonBP/Blueprints/FirstPersonCharacter` (`GameplayStatics.GetPlayerCharacter` 0)))
  (if (== (`/Game/FirstPersonBP/Blueprints/FirstPersonCharacter.Sphere` _asfirst_person_character) OtherComp)
    (`/Game/HazardBP/Effects/EffectBP.Begin Effect` (`/Game/FirstPersonBP/Blueprints/FirstPersonCharacter.Effect_Freeze_LargeBarrel` _asfirst_person_character))))

(event `self.Explosion_Volume.OnComponentEndOverlap`
  (params (OverlappedComponent :type "PrimitiveComponent Object Reference") (OtherActor :type "Actor Object Reference") (OtherComp :type "PrimitiveComponent Object Reference") (OtherBodyIndex :type Integer))
  ;[1 1 1] When the player is affected by the explostion
  (bind _asfirst_person_character (cast `/Game/FirstPersonBP/Blueprints/FirstPersonCharacter` (`GameplayStatics.GetPlayerCharacter` 0)))
  (if (or (== (`/Game/FirstPersonBP/Blueprints/FirstPersonCharacter.Sphere` _asfirst_person_character) OtherComp) (== "/Game/FirstPersonBP/Blueprints/FirstPersonProjectile.FirstPersonProjectile" OtherComp))
    (`/Game/HazardBP/Effects/EffectBP.Begin Effect` (`/Game/FirstPersonBP/Blueprints/FirstPersonCharacter.Effect_Freeze_LargeBarrel` _asfirst_person_character))))

(fn `UserConstructionScript`)