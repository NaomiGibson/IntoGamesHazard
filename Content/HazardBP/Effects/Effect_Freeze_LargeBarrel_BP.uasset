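; Freeze effect for the large barrel hazard that damages the first-person character, built as a child of a shared effect Blueprint.
; BeginEffect runs the parent logic, then applies InitialDamage if IsEffectActive is false.
; DuringEffect runs the parent logic, prints DamagePerFrequency as debug output, then applies it as damage.
; Any freeze behavior beyond damage is not defined in this graph.
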(fn `Begin Effect`
  (`parent.Begin Effect`)
  (if (not (`self.IsEffectActive`))
    (`/Game/FirstPersonBP/Blueprints/FirstPersonCharacter.TakeDamage` (`self.As First Person Character`) (`self.InitialDamage`))))

(fn `During Effect`
  (`parent.During Effect`)
  (`KismetSystemLibrary.PrintString` (`KismetStringLibrary.Conv_IntToString` (`self.DamagePerFrequency`)))
  ;[1 1 1] Inflicts damage
  (`/Game/FirstPersonBP/Blueprints/FirstPersonCharacter.TakeDamage` (`self.As First Person Character`) (`self.DamagePerFrequency`)))