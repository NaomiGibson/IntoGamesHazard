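; Effect_BP is an effect base that manages a timed or continual effect, caching its owner as a FirstPersonCharacter on BeginPlay.
; BeginEffect sets the remaining duration and starts a looping DuringEffect timer, using Frequency as the interval.
; When HasDuration is set, each tick of that timer subtracts 1/Frequency and calls EndEffect below zero to clear the timer.
; No damage is applied in these graphs.
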(event `self.ReceiveBeginPlay`
  (bind _asfirst_person_character (cast `/Game/FirstPersonBP/Blueprints/FirstPersonCharacter` (`self.GetOwner`)))
  (set `self.As First Person Character` _asfirst_person_character))

(fn `Begin Effect`
  ;[1 1 1] Sets up timer for duration / continual damage
  (if (`self.HasDuration`)
    (set `self.DurationRemaining` (`KismetMathLibrary.Conv_IntToDouble` (`self.Duration`))))
  (bind _returnvalue (`KismetSystemLibrary.K2_SetTimer` null "DuringEffect" (`self.Frequency`) true))
  (set `self.DuringEffectTimer` _returnvalue))

(fn `During Effect`
  (if (`self.HasDuration`)
    (bind _output_get (set `self.DurationRemaining` (- (`self.DurationRemaining`) (/ 1.0 (`self.Frequency`)))))
    (if (< _output_get 0.0)
      (`self.End Effect`))))

(fn `End Effect`
  (`KismetSystemLibrary.K2_ClearAndInvalidateTimerHandle` (`self.DuringEffectTimer`)))