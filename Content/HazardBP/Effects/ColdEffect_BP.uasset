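; ColdEffect_BP is a cold status effect for its owning FirstPersonCharacter that displays a frostbite screen overlay.
; BeginPlay creates the FreezeEffect_UI widget, and BeginEffect shows its overlay and starts a looping timer at Frequency, refreshing only the duration if already active.
; For timed effects, each DuringEffect tick subtracts Frequency and calls EndEffect when the remainder exactly equals zero, hiding the overlay and clearing the timer.
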(event `self.ReceiveBeginPlay`
  (bind _asfirst_person_character (cast `/Game/FirstPersonBP/Blueprints/FirstPersonCharacter` (`self.GetOwner`)))
  (set `self.As First Person Character` _asfirst_person_character)
  (bind _returnvalue (`|CreateWidget` "/Game/HazardBP/UI/FreezeEffect_UI.FreezeEffect_UI_C"))
  (set `self.Frostbite_UI` _returnvalue)
  (`UserWidget.AddToPlayerScreen` _returnvalue 0))

(fn `Begin Effect`
  ;[1 1 1] Cold UI effect is visible
  (`Widget.SetVisibility` (`/Game/HazardBP/UI/FreezeEffect_UI.Fostbite_OverlayImage` (`self.Frostbite_UI`)) "Visible")
  ;[1 1 1] Ensures the duration period is reset if the effect is already active
  (if (`self.HasDuration`)
    (set `self.DurationRemaining` (`KismetMathLibrary.Conv_IntToDouble` (`self.Duration`))))
  ;[1 1 1] Begin the repeating effect happening at the given frequency
  (if (not (`self.IsEffectActive`))
    (bind _returnvalue (`KismetSystemLibrary.K2_SetTimer` null "During Effect" (`self.Frequency`) true))
    (set `self.DuringEffectTimer` _returnvalue)
    (set `self.IsEffectActive` true)))

(fn `During Effect`
  (if (`self.HasDuration`)
    ;[1 1 1] Counts down the duration period
    (bind _output_get (set `self.DurationRemaining` (- (`self.DurationRemaining`) (/ (`self.Frequency`) 1.0))))
    ;[1 1 1] Once the duration period is over, the effect is ended
    (if (== _output_get 0.0)
      (`self.End Effect`))))

(fn `End Effect`
  ;[1 1 1] remove the frost UI effect
  (`Widget.SetVisibility` (`/Game/HazardBP/UI/FreezeEffect_UI.Fostbite_OverlayImage` (`self.Frostbite_UI`)) "Hidden")
  (`KismetSystemLibrary.K2_ClearAndInvalidateTimerHandle` (`self.DuringEffectTimer`))
  (set `self.IsEffectActive` false))