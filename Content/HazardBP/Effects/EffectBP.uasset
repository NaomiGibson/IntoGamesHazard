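; EffectBP is a component on the first-person character that drives a timed frostbite screen effect.
; On BeginPlay it adds a FreezeEffect_UI widget to the player screen.
; BeginEffect shows the overlay and starts a looping timer that replays the frost damage animation; retriggering refreshes the duration without restarting the timer.
; With a duration set, each tick counts down and calls EndEffect at exactly zero, hiding the overlay and clearing the timer.
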(event `self.ReceiveBeginPlay`
  (bind _asfirst_person_character (cast `/Game/FirstPersonBP/Blueprints/FirstPersonCharacter` (`self.GetOwner`)))
  (set `self.As First Person Character` _asfirst_person_character)
  (bind _returnvalue (`|CreateWidget` "/Game/HazardBP/UI/FreezeEffect_UI.FreezeEffect_UI_C"))
  (set `self.Frostbite_UI` _returnvalue)
  (`UserWidget.AddToPlayerScreen` _returnvalue 0))

(fn `Begin Effect`
  (bind _frostbite_ui (`self.Frostbite_UI`))
  (`Widget.SetVisibility` (`/Game/HazardBP/UI/FreezeEffect_UI.Fostbite_OverlayImage` (`self.Frostbite_UI`)) "Visible")
  (`UserWidget.PlayAnimation` _frostbite_ui (`/Game/HazardBP/UI/FreezeEffect_UI.ExplosionDamage` _frostbite_ui) 0.0 1 "Forward" 1.0 true)
  (if (`self.HasDuration`)
    (set `self.DurationRemaining` (`KismetMathLibrary.Conv_IntToDouble` (`self.Duration`))))
  (if (not (`self.IsEffectActive`))
    ;[1 1 1] Sets up timer for duration / continual damage
    (bind _returnvalue (`KismetSystemLibrary.K2_SetTimer` null "During Effect" (`self.Frequency`) true))
    (set `self.DuringEffectTimer` _returnvalue)
    (set `self.IsEffectActive` true)))

(fn `During Effect`
  (bind _frostbite_ui (`self.Frostbite_UI`))
  (`UserWidget.PlayAnimation` _frostbite_ui (`/Game/HazardBP/UI/FreezeEffect_UI.FrostDamage` _frostbite_ui) 0.0 1 "Forward" 1.0 true)
  (if (`self.HasDuration`)
    (bind _output_get (set `self.DurationRemaining` (- (`self.DurationRemaining`) (/ (`self.Frequency`) 1.0))))
    (if (== _output_get 0.0)
      (`self.End Effect`))))

(fn `End Effect`
  (`Widget.SetVisibility` (`/Game/HazardBP/UI/FreezeEffect_UI.Fostbite_OverlayImage` (`self.Frostbite_UI`)) "Hidden")
  (set `self.IsEffectActive` false)
  (`KismetSystemLibrary.K2_ClearAndInvalidateTimerHandle` (`self.DuringEffectTimer`)))