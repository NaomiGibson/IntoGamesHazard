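; Frostbite status effect Blueprint that trades periodic damage to the first-person character for a temporary Strength boost.
; It overrides the parent effect's begin, during and end hooks, calling the parent each time.
; Begin adds StrengthIncrease to the character's Strength, During applies DamagePerFrequency as damage, and End subtracts the same increase.
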(fn `Begin Effect`
  (bind _as_first_person_character (`self.As First Person Character`))
  (`parent.Begin Effect`)
  ;[1 1 1] Increase strength
  (set `/Game/FirstPersonBP/Blueprints/FirstPersonCharacter.Strength` (+ (`/Game/FirstPersonBP/Blueprints/FirstPersonCharacter.Strength` _as_first_person_character) (`self.StrengthIncrease`)) _as_first_person_character))

(fn `During Effect`
  (`parent.During Effect`)
  ;[1 1 1] Take damage
  (`/Game/FirstPersonBP/Blueprints/FirstPersonCharacter.TakeDamage` (`self.As First Person Character`) (`self.DamagePerFrequency`)))

(fn `End Effect`
  (bind _as_first_person_character (`self.As First Person Character`))
  (`parent.End Effect`)
  (set `/Game/FirstPersonBP/Blueprints/FirstPersonCharacter.Strength` (- (`/Game/FirstPersonBP/Blueprints/FirstPersonCharacter.Strength` _as_first_person_character) (`self.StrengthIncrease`)) _as_first_person_character))