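; Freeze hazard effect for the small barrel that damages the affected first-person character.
; It extends a parent effect, calling the parent logic in both overrides before applying damage.
; Begin Effect deals the initial damage, and During Effect deals the per-frequency damage.
; The file itself adds no slowing or visual freeze behavior, and its BeginPlay and Tick events are disabled.
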(fn `Begin Effect`
  (`parent.Begin Effect`)
  (`/Game/FirstPersonBP/Blueprints/FirstPersonCharacter.TakeDamage` (`self.As First Person Character`) (`self.InitialDamage`)))

(fn `During Effect`
  (`parent.During Effect`)
  (`/Game/FirstPersonBP/Blueprints/FirstPersonCharacter.TakeDamage` (`self.As First Person Character`) (`self.DamagePerFrequency`)))