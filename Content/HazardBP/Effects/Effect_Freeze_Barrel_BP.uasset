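; Freeze barrel effect Blueprint that deals frost damage to the first-person character and shows it on the Frostbite UI.
; When the effect begins, it applies initial damage and plays the explosion damage animation.
; While the effect runs, it applies frostbite damage and plays the frost damage animation.
; Both steps extend the parent effect's functions, calling the parent version before adding the damage and UI feedback.
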(event `self.ReceiveBeginPlay`
  (`parent.ReceiveBeginPlay`))

(fn `Begin Effect`
  (bind _frostbite_ui (`self.Frostbite_UI`))
  (`parent.Begin Effect`)
  (`/Game/FirstPersonBP/Blueprints/FirstPersonCharacter.TakeDamage` (`self.As First Person Character`) (`self.InitialDamage`))
  (`UserWidget.PlayAnimation` _frostbite_ui (`/Game/HazardBP/UI/FreezeEffect_UI.ExplosionDamage` _frostbite_ui) 0.0 1 "Forward" 1.0 true))

(fn `During Effect`
  (bind _frostbite_ui (`self.Frostbite_UI`))
  (`parent.During Effect`)
  (`/Game/FirstPersonBP/Blueprints/FirstPersonCharacter.TakeDamage` (`self.As First Person Character`) (`self.FrostbiteDamageDamage`))
  (`UserWidget.PlayAnimation` _frostbite_ui (`/Game/HazardBP/UI/FreezeEffect_UI.FrostDamage` _frostbite_ui) 0.0 1 "Forward" 1.0 true))