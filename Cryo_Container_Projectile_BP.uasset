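; Thrown cryo container projectile that launches itself on spawn, explodes and then removes itself.
; BeginPlay sets forward velocity and adds a velocity-based impulse, then timed delays spawn a scaled explosion emitter and destroy the actor.
; A follow-up impulse targets the emitter component instead of surrounding objects and is marked as not working.
; Overlapping the container calls InteractCryoContainer on the first-person character.
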(event `self.CryoContainer.OnComponentBeginOverlap`
  (params (OverlappedComponent :type "PrimitiveComponent Object Reference") (OtherActor :type "Actor Object Reference") (OtherComp :type "PrimitiveComponent Object Reference") (OtherBodyIndex :type Integer) (bFromSweep :type Boolean) (SweepResult :type "HitResult Structure (by ref)"))
  ;[1 1 1] Allows First Person Interaction
  (bind _asfirst_person_character (cast `/Game/FirstPersonBP/Blueprints/FirstPersonCharacter` OtherActor))
  (`/Game/FirstPersonBP/Blueprints/FirstPersonCharacter.Interact_CryoContainer` _asfirst_person_character))

(event `self.ReceiveBeginPlay`
  (bind _cryocontainer (`self.CryoContainer`))
  ;[1 1 1] Throws Cryo Container
  (`PrimitiveComponent.SetPhysicsLinearVelocity` _cryocontainer (* (`SceneComponent.GetForwardVector` _cryocontainer) 500) false "None")
  ;;[1 1 1] Makes Items move In Game
  (`PrimitiveComponent.AddImpulseAtLocation` _cryocontainer (* (`self.GetVelocity`) 200.0) (`self.K2_GetActorLocation`) "None")
  ;;[1 1 1] Cause Explosion
  (`KismetSystemLibrary.Delay` 2.0)
  (bind _returnvalue (`GameplayStatics.SpawnEmitterAtLocation` "/Game/StarterContent/Particles/P_Explosion.P_Explosion" (`SceneComponent.K2_GetComponentLocation` _cryocontainer) (struct) (4.0 4.0 4.0)))
  ;;[1 1 1] Makes Explosion Move Objects (Currently not working)
  (`PrimitiveComponent.AddImpulseAtLocation` _returnvalue (* (`self.GetVelocity`) 400.0) (`self.K2_GetActorLocation`) "None")
  (`KismetSystemLibrary.Delay` 2.0)
  (`self.K2_DestroyActor`) ; Destroys Cryo Container
)

(fn `UserConstructionScript`)